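; BP_Target_Cube1 is a moving target cube that briefly flashes green when it takes any damage.
; Damage swaps the cube's material to green, and a retriggerable delay restores red shortly after the last hit.
; A timeline started on BeginPlay drives the cube's relative location; a delay on its Update pin periodically toggles IsLooped to alternate between Play and Reverse, moving it back and forth.
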(event EventBeginPlay
  (bind _moving (Timeline|Timeline_0 Play)
    (:Update
      (Transformation|SetRelativeLocation (Variables|Default|GetCube) _moving false false)
      (Utilities|FlowControl|Delay 4.0)
      (if (Variables|Default|GetIsLooped)
        (Variables|Default|SetIsLooped false)
        (Timeline|Timeline_0 Reverse)
        (else
          (Variables|Default|SetIsLooped true)
          (Timeline|Timeline_0 Play))))))

(event Game|Damage|EventAnyDamage
  (params (Damage :type Float%20%28single-precision%29) (DamageType :type Damage%20Type%20Object%20Reference) (InstigatedBy :type Controller%20Object%20Reference) (DamageCauser :type Actor%20Object%20Reference))
  (Rendering|Material|SetMaterial (Variables|Default|GetCube) 0 "/Game/Materials/TargetMaterials/M_Targ_Green.M_Targ_Green")
  (Utilities|FlowControl|RetriggerableDelay 0.5)
  (Rendering|Material|SetMaterial (Variables|Default|GetCube) 0 "/Game/Materials/TargetMaterials/M_Targ_Red.M_Targ_Red"))

(fn ConstructionScript
  (|CallParentFunction))