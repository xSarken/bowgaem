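; BP_BaseArrow is the base bow arrow projectile, which damages and sticks into what it hits.
; Its projectile velocity is zeroed on BeginPlay so it does not fly away on spawn.
; On hit, it pushes physics-simulating components with an impulse from its velocity and has them ignore it when moving.
; Every hit applies speed-scaled damage, then attaches the arrow to the hit bone with a random forward nudge to embed it.
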(event EventBeginPlay
  ;[1 1 1] Making arrow not fly away on spawn
  (Variables|/Script/Engine.MovementComponent|SetVelocity (Variables|Default|GetProjectileMovement) "0, 0, 0"))

(event Collision|EventHit
  (params (MyComp :type Primitive%20Component%20Object%20Reference) (Other :type Actor%20Object%20Reference) (OtherComp :type Primitive%20Component%20Object%20Reference) (bSelfMoved :type Boolean) (HitLocation :type Vector :default "0, 0, 0") (HitNormal :type Vector :default "0, 0, 0") (NormalImpulse :type Vector :default "0, 0, 0") (Hit :type Hit%20Result%20Structure%20%28by%20ref%29))
  ;[1 1 1] Adding arrow power to objects it hits
  (if (Physics|IsSimulatingPhysics OtherComp "None")
    (Utilities|FlowControl|Sequence
      (:then_0
        (Physics|AddImpulseatLocation OtherComp (Transformation|GetComponentVelocity MyComp) HitLocation "None")
        (Collision|IgnoreActorwhenMoving OtherComp self true))
      (:then_1
        (bind _output_get (Variables|Default|SetHitVelocityLength (Math|Vector|VectorLength (Transformation|GetComponentVelocity MyComp)) :!label _label))
        ;[1 1 1] Applies damage based on arrow speed
        (Game|Damage|ApplyDamage Other (* _output_get 0.024) 0 0)
        ;[1 1 1] Attach the arrow to object
        (Transformation|AttachComponentToComponent OtherComp (.HitBoneName (Collision|BreakHitResult Hit)) "KeepWorld" "KeepWorld" "KeepWorld" true)
        (Transformation|AddActorLocalOffset (Math|Vector|MakeVector (Math|Random|RandomFloatinRange 1e+01 2e+01) 0.0 0.0) false true)))
    (else
      (goto _label))))

(fn ConstructionScript)