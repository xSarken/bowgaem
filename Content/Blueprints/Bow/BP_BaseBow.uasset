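; Base grabbable bow that is held with one component, drawn with a second, and fires arrow projectiles.
; The first Pickup attaches the bow; a second near the string socket sets the string component and spawns an attached arrow.
; Tick derives Charge from pull distance in socket space and aims the bow along the line between both components.
; AltRelease launches the arrow at curve-mapped speed; Release drops the bow with physics.
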(event EventAltRelease
  ;[0.9341 1 0.9798] Shoot arrow
  (Variables|Default|SetStringComp 0)
  (Transformation|AttachComponentToComponent (Variables|Default|GetGrabComp) "None" "SnapToTarget" "SnapToTarget" "KeepWorld" true)
  (bind _arrow (Variables|Default|GetArrow)
    (:then
      (Transformation|DetachFromActor _arrow "KeepWorld" "KeepWorld" "KeepWorld")
      (Variables|/Script/Engine.ProjectileMovementComponent|SetProjectileGravityScale (Variables|/Game/Blueprints/Bow/BP_BaseArrow.BP_BaseArrow_C|GetProjectileMovement _arrow) 1.0)
      (Variables|/Script/Engine.MovementComponent|SetVelocity (Variables|/Game/Blueprints/Bow/BP_BaseArrow.BP_BaseArrow_C|GetProjectileMovement _arrow) (* (Transformation|GetActorForwardVector _arrow) (Math|Float|MapRangeClamped (Math|Curves|GetFloatValue (Variables|Default|GetFloatCurve) (Variables|Default|GetCharge)) 0.0 1.0 25.0 3e+03)))
      (Variables|/Script/Engine.ProjectileMovementComponent|SetbRotationFollowsVelocity (Variables|/Game/Blueprints/Bow/BP_BaseArrow.BP_BaseArrow_C|GetProjectileMovement _arrow) true)
      (Variables|Default|SetArrow 0)
      (Transformation|SetActorRelativeRotation "0, 0, 0"))
    (:else
      _))
  (Variables|Default|SetCharge 0.0))

(event EventPickup
  (params (AttachTo :type Scene%20Component%20Object%20Reference))
  ;[1 1 1] Grab
  (Variables|Default|GetGrabComp
    (:then
      (if (< (Math|Vector|VectorLength (- (Transformation|GetWorldLocation AttachTo) (Transformation|GetSocketLocation (Variables|Default|GetSkeletalMesh) "string1"))) 2e+01)
        (Variables|Default|SetStringComp AttachTo)
        (bind _returnvalue (Game|SpawnActorfromClass (Variables|Default|GetArrowProjectileClass) (Transformation|GetWorldTransform (Variables|Default|GetSkeletalMesh)) "Undefined" 0 0))
        (bind _output_get (Variables|Default|SetArrow _returnvalue))
        ;;[1 1 1] Attach Arrow
        (Transformation|AttachComponentToComponent _output_get (Variables|Default|GetSkeletalMesh) "bowString" "KeepWorld" "KeepWorld" "KeepWorld" true)
        (Transformation|AddActorLocalOffset _output_get "20.000000, 0, 0" false false)))
    (:else
      (bind _output_get_2 (Variables|Default|SetGrabComp AttachTo))
      (Transformation|AttachComponentToComponent _output_get_2 "None" "SnapToTarget" "SnapToTarget" "KeepWorld" true)
      (Collision|SetCollisionEnabled (Variables|Default|GetSkeletalMesh) "QueryOnly"))))

(event EventRelease
  ;[1 1 1] Release/ Drop
  (Transformation|DetachFromActor "KeepWorld" "KeepWorld" "KeepWorld")
  (Variables|Default|SetStringComp 0)
  (Variables|Default|SetGrabComp 0)
  (Variables|Default|SetCharge 0.0)
  (Collision|SetCollisionEnabled (Variables|Default|GetSkeletalMesh) "QueryAndPhysics")
  (Physics|SetSimulatePhysics (Variables|Default|GetSkeletalMesh) true))

(event EventTick
  (params (DeltaSeconds :type Float%20%28single-precision%29))
  (bind _grabcomp (Variables|Default|GetGrabComp))
  (bind _stringcomp (Variables|Default|GetStringComp))
  (bind _returnvalue (Transformation|GetWorldLocation _grabcomp))
  (bind _returnvalue_2 (Transformation|GetWorldLocation _stringcomp))
  (bind _returnvalue_3 (Math|Rotator|FindLookatRotation _returnvalue_2 _returnvalue))
  (bind (_roll _pitch _yaw) (Math|Rotator|BreakRotator _returnvalue_3))
  ;[1 1 1] Allowing to grab string and bow
  ;;[1 1 1] String location comparison
  (bind _stringcomp_2 (Variables|Default|GetStringComp)
    (:then
      (Variables|Default|SetCharge (* (Math|Float|MapRangeClamped (Math|Float|Clamp(Float) (.x (Math|Transform|InverseTransformLocation (Transformation|GetSocketTransform (Variables|Default|GetSkeletalMesh) "string1" "RTS_World") (Transformation|GetWorldLocation _stringcomp_2))) -35.0 0.0) -35.0 0.0 -1.0 0.0) -1.0))
      ;;[1 1 1] Aiming
      (Transformation|SetActorRotation (Math|Rotator|MakeRotator (.roll (Transformation|GetWorldRotation _grabcomp)) _pitch _yaw)))
    (:else)))

(fn ConstructionScript)